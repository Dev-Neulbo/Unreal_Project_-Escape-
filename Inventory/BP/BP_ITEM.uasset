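; BP_ITEM is an item actor that can be added to the player's inventory.
; Its construction script looks up the row from ItemImport's data table handle, stores it in ItemSA and applies its mesh.
; ClickE appends the item's code to the Inventory array on BP_GameInstance, then prints the first two entries as debug output.
; The actor is not destroyed on pickup, and its event graph is empty.
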(fn `Click_E`
  (bind _output_get (set `self.ItemRowName` (`.ItemCode_9_6B6DF9B74C0D3528FDD7009EB6C9BF16` (break `/Game/Inventory/Struct/ST_Item` (`self.Item_SA`)))))
  (bind _asbp_game_instance (cast `/Game/Inventory/Instance/BP_GameInstance` (`GameplayStatics.GetGameInstance`)))
  (bind _inventory (`/Game/Inventory/Instance/BP_GameInstance.Inventory` _asbp_game_instance))
  (`KismetArrayLibrary.Array_Add` _inventory _output_get)
  (`KismetSystemLibrary.PrintString` (`KismetStringLibrary.Conv_NameToString` (`|GetArrayItem` _inventory)))
  (`KismetSystemLibrary.PrintString` (`KismetStringLibrary.Conv_NameToString` (`|GetArrayItem` _inventory 1))))

(fn `UserConstructionScript`
  (locals (NewLocalVar :type " Structure"))
  (bind (_datatable _rowname) (break `DataTableRowHandle` (`.Item_Handle_2_3CFF4F1042F7DAB76C5031829CB8BEB6` (break `/Game/Inventory/Struct/ST_Item_Handle` (`self.Item_Import`)))))
  (bind _returnvalue (`|GetDataTableRow` _datatable _rowname)
    (:`then`
      (set `self.Item_SA` _returnvalue)
      (`StaticMeshComponent.SetStaticMesh` (`self.StaticMesh`) (`.Mesh_18_54D1C4614EA89901FAE0559E9551092B` (break `/Game/Inventory/Struct/ST_Item` _returnvalue))))))